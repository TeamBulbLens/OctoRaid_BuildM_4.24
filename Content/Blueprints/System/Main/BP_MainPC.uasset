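; Main-game player controller for an asymmetric match between a VR octopus and on-screen hunters, choosing the role from headset detection.
; On local BeginPlay it streams the game sublevel, then sets up each role's pawn and HUD.
; The server gathers player HP and relays HUD, loading and result updates through every controller, while the octopus gets controller-attached and pawn widgets.
; It also handles restart, lobby return and debug keys.
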(event Custom|ShowResultHunters
  (params (bIsHunterVictory :type Boolean))
  ;[1 1 1] 결과 출력
  ;;[1 1 1] 헌터 결과 UI표시
  ;; 서버의 헌터UI를 표시하는 것이 아니므로 소유 클라이언트에서 실행
  (if (Utilities|IsLocalHunter?)
    (bind _returnvalue (UserInterface|CreateWidget "/Game/Blueprints/System/Main/HunterResultWidget.HunterResultWidget_C"))
    (UserInterface|Viewport|AddtoViewport _returnvalue 0)
    (Default|ShowResult _returnvalue bIsHunterVictory)))

(event Custom|EndLoadingMulticast
  ;[1 1 1] 로딩
  ;;[1 1 1] 로딩 끝내기 : 로딩 UI 제거하고 폰 배치
  (CallFunction|EndLoading))

(event Custom|UpdateHunterMainWidgetClient
  (params (PlayerCurrentHP :type Array%20of%20Player%20HP%20Data%20Structures) (LogOutUIDs :type Array%20of%20Integers))
  ;[1 1 1] 헌터 UI 업데이트
  (CallFunction|UpdateWidget PlayerCurrentHP LogOutUIDs))

(event Custom|LoadGameMap
  ;[1 1 1] 로딩
  ;;[1 1 1] 맵 로딩 함수들
  (bind _asbp_main_gs (Utilities|Casting|CastToBP_MainGS (Game|GetGameState)))
  (if (Utilities|Enum|Equal(Enum) (Variables|/Script/OctoPrototype.MainGS|GetCurrentGameState _asbp_main_gs) "Initialize")
    (Variables|/Script/OctoPrototype.MainGS|SetCurrentGameState _asbp_main_gs "Loading")
    (Class|MainGS|DowhenCurrentGameStateChanged _asbp_main_gs)
    (Game|LoadStreamLevel(byName) "Game_SubLevel" true)
    (CallFunction|EndLoading)))

(event Custom|EndLoadingServer
  ;[1 1 1] 로딩
  ;;[1 1 1] 로딩 끝내기 : 로딩 UI 제거하고 폰 배치
  (CallFunction|EndLoadingMulticast))

(event Custom|ShowResult
  (params (bIsHunterVictory :type Boolean))
  ;[1 1 1] 결과 출력
  (CallFunction|ShowResultServer bIsHunterVictory)
  (CallFunction|ShowResulttoClients bIsHunterVictory))

(event Custom|UpdateRespawnCount
  (bind _huntermainwidget (Variables|Default|GetHunterMainWidget))
  ;[1 1 1] 헌터 UI 업데이트
  (bind _asbp_main_gs (Utilities|Casting|CastToBP_MainGS (Game|GetGameState)))
  (Utilities|IsValid _asbp_main_gs
    (:Is%20Valid
      (Utilities|IsValid _huntermainwidget
        (:Is%20Valid
          (Default|SetRespawnCount _huntermainwidget (Variables|/Game/Blueprints/System/Main/BP_MainGS.BP_MainGS_C|GetRespawnCount _asbp_main_gs)))))))

(event Custom|PawnSpawn
  (params (Pawn :type Pawn%20Object%20Reference))
  ;[1 1 1] 로딩
  ;;[1 1 1] 로딩 끝내기 : 로딩 UI 제거하고 폰 배치
  (bind _asbp_main_gm (Utilities|Casting|CastToBP_MainGM (Game|GetGameMode)))
  (Default|RespawnPawn _asbp_main_gm Pawn))

(event Custom|ShowLoading
  ;[1 1 1] 로딩
  ;;[1 1 1] 헌터 로딩 UI 표시
  ;; 서버의 헌터UI를 표시하는 것이 아니므로 소유 클라이언트에서 실행
  (if (Utilities|IsLocalHunter?)
    (Viewport|RemoveAllWidgets)
    (bind _returnvalue (UserInterface|CreateWidget "/Game/Blueprints/System/Public/LoadingWidget.LoadingWidget_C"))
    (UserInterface|Viewport|AddtoViewport _returnvalue 0)
    (Variables|Default|SetbShowMouseCursor false)
    (Input|SetInputModeUIOnly self 0 "DoNotLock")))

(event Custom|UpdateOctoWidgetServer
  (bind _octomainwidget (Variables|Default|GetOctoMainWidget))
  ;[1 1 1] 헌터 UI 업데이트
  (bind _asbp_main_ps (Utilities|Casting|CastToBP_MainPS (Variables|GetPlayerState)))
  (Utilities|IsValid _asbp_main_ps
    (:Is%20Valid
      (Utilities|IsValid _octomainwidget
        (:Is%20Valid
          (bind _maxhp (Default|GetMaxHP _asbp_main_ps))
          (Default|SetOctoHPBarPercent _octomainwidget (/ (Variables|/Game/Blueprints/System/Main/BP_MainPS.BP_MainPS_C|GetCurrentHP _asbp_main_ps) _maxhp)))))))

(event Custom|UpdateOctoRespawnCount
  (bind _octomainwidget (Variables|Default|GetOctoMainWidget))
  ;[1 1 1] 헌터 UI 업데이트
  (bind _asbp_main_gs (Utilities|Casting|CastToBP_MainGS (Game|GetGameState)))
  (Utilities|IsValid _asbp_main_gs
    (:Is%20Valid
      (Utilities|IsValid _octomainwidget
        (:Is%20Valid
          (Default|SetRespawnCount _octomainwidget (Variables|/Game/Blueprints/System/Main/BP_MainGS.BP_MainGS_C|GetRespawnCount _asbp_main_gs)))))))

(event Custom|HideOctoMainWidget
  (bind _octomainwidget (Variables|Default|GetOctoMainWidget))
  ;[1 1 1] 문어 UI 위젯 추가
  (Utilities|IsValid _octomainwidget
    (:Is%20Valid
      (Widget|SetVisibility _octomainwidget "Collapsed"))))

(event Custom|GoToLobby
  ;[1 1 1] 로딩
  ;;[1 1 1] 맵 로딩 함수들
  (CallFunction|HideOctoMainWidget)
  (CallFunction|ShowLoadingtoClients)
  (bind _asbp_gi (Utilities|Casting|CastToBP_GI (Game|GetGameInstance)))
  (Default|BacktoLobby _asbp_gi))

(event Custom|LogOutSubWidget
  (params (UID :type Integer))
  ;[1 1 1] 헌터 UI 업데이트
  (Utilities|Array|Add (Variables|Default|GetLogOutUIDs) UID)
  (CallFunction|UpdateHunterMainWidgetServer))

(event Custom|RestartGame
  ;[1 1 1] 로딩
  ;;[1 1 1] 맵 로딩 함수들
  (CallFunction|HideOctoMainWidget)
  (CallFunction|ShowLoadingtoClients)
  (bind _asbp_gi (Utilities|Casting|CastToBP_GI (Game|GetGameInstance)))
  (Default|StartMainGame _asbp_gi 1.0))

(event Custom|SetMeshAndMaterialAllPlayersServer
  ;[1 1 1] 캐릭터 스킨 설정
  (Utilities|IsValid (Game|GetGameMode)
    (:Is%20Valid
      (Utilities|FlowControl|Delay 2.0)
      (bind _outactors (Actor|GetAllActorsOfClass "/Game/Blueprints/System/Main/BP_MainPS.BP_MainPS_C"))
      (for _array_element _outactors
        (Default|SetMeshandMaterial _array_element)))))

(event Custom|AddOctoMainWidget
  ;[1 1 1] 문어 UI 위젯 추가
  (bind _asbp_vrpawn_main (Utilities|Casting|CastToBP_VRPawnMain (Pawn|GetControlledPawn)))
  (Utilities|IsValid _asbp_vrpawn_main
    (:Is%20Valid
      (Utilities|IsValid (Variables|Default|GetOctoMainWidget)
        (:Is%20Valid
          (CallFunction|UpdateOctoRespawnCount))
        (:Is%20Not%20Valid
          (bind _returnvalue (Game|SpawnActorfromClass "/Game/Blueprints/System/Main/BP_OctoMainWidget.BP_OctoMainWidget_C" (Transformation|GetWorldTransform (Variables|/Game/Blueprints/Octopus/BP_MotionControllerMain.BP_MotionControllerMain_C|GetMotionController (Variables|/Game/Blueprints/Octopus/BP_VRPawnMain.BP_VRPawnMain_C|GetLeftController _asbp_vrpawn_main))) "AlwaysSpawn" _asbp_vrpawn_main 0))
          (Transformation|AttachComponentToComponent _returnvalue (Variables|/Game/Blueprints/Octopus/BP_MotionControllerMain.BP_MotionControllerMain_C|GetMotionController (Variables|/Game/Blueprints/Octopus/BP_VRPawnMain.BP_VRPawnMain_C|GetLeftController _asbp_vrpawn_main)) "None" "SnapToTarget" "SnapToTarget" "KeepWorld" true)
          (bind _asocto_main_widget (Utilities|Casting|CastToOctoMainWidget (UserInterface|GetUserWidgetObject (Variables|/Game/Blueprints/System/Main/BP_OctoMainWidget.BP_OctoMainWidget_C|GetWidget _returnvalue))))
          (Variables|Default|SetOctoMainWidget _asocto_main_widget)
          (Default|AttachUnderWaterWidgert _asbp_vrpawn_main))))))

(event Custom|ShowResultToClients
  (params (bIsHunterVictory :type Boolean))
  ;[1 1 1] 결과 출력
  ;;[1 1 1] 헌터 결과 UI 표시 지시
  ;; 서버가 가지고 있는 헌터들의 플레이어 콘트롤러에 foreach로 각각 uI를 표시하라고 지시한다
  (Utilities|IsValid (Game|GetGameMode)
    (:Is%20Valid
      (bind _outactors (Actor|GetAllActorsOfClass "BP_MainPC_C"))
      (for _array_element _outactors
        (CallFunction|ShowResultHunters _array_element bIsHunterVictory)))))

(event Custom|ShowResultServer
  (params (bIsHunterVictory :type Boolean))
  ;[1 1 1] 결과 출력
  ;;[1 1 1] VR 쪽 결과화면 표시
  (Utilities|IsValid (Game|GetGameMode)
    (:Is%20Valid
      (bind _asbp_vrpawn_main (Utilities|Casting|CastToBP_VRPawnMain (Game|Player|GetPlayerPawn 0)))
      (Utilities|IsValid _asbp_vrpawn_main
        (:Is%20Valid
          (Default|SetResultUI _asbp_vrpawn_main "Visible")
          (Default|ShowResult (Variables|/Game/Blueprints/Octopus/BP_VRPawnMain.BP_VRPawnMain_C|GetOctoResultWidget _asbp_vrpawn_main) bIsHunterVictory))))))

(event Custom|UpdateHunterMainWidgetServer
  ;[1 1 1] 헌터 UI 업데이트
  (CallFunction|SyncPlayerCurrentHPServer)
  (CallFunction|UpdateHunterWidgettoClient (Variables|Default|GetLogOutUIDs))
  (CallFunction|UpdateRespawnCount)
  (CallFunction|UpdateOctoWidgetServer)
  (CallFunction|UpdateOctoRespawnCount))

(event Custom|ShowLoadingToClients
  ;[1 1 1] 로딩
  ;;[1 1 1] 헌터 로딩 UI 표시 지시
  ;; 서버가 가지고 있는 헌터들의 플레이어 콘트롤러에 foreach로 각각 uI를 표시하라고 지시한다
  (Utilities|IsValid (Game|GetGameMode)
    (:Is%20Valid
      (bind _outactors (Actor|GetAllActorsOfClass "BP_MainPC_C"))
      (for _array_element _outactors
        (CallFunction|ShowLoading _array_element)))))

(event EventBeginPlay
  ;[1 1 1] 초기화
  (if (Pawn|IsLocalPlayerController)
    (CallFunction|LoadGameMap)
    (if (Utilities|IsLocalHunter?)
      (Variables|Default|SetbShowMouseCursor false)
      (Input|SetInputModeUIOnly self 0 "DoNotLock")
      (Utilities|Array|Clear (Variables|Default|GetLogOutUIDs)))))

(event Input|KeyboardEvents|F1
  (params (Key :type Key%20Structure))
  ;[1 0.8557 0] for debug
  (:Pressed
    (bind _asbp_gi (Utilities|Casting|CastToBP_GI (Game|GetGameInstance)))
    (Variables|/Game/Blueprints/Public/BP_GI.BP_GI_C|SetIsDebugMode _asbp_gi (not (Variables|/Game/Blueprints/Public/BP_GI.BP_GI_C|GetIsDebugMode _asbp_gi)))))

(event Input|KeyboardEvents|Enter
  (params (Key :type Key%20Structure))
  ;[1 0.8557 0] for debug
  (:Pressed
    (bind _asbp_gi (Utilities|Casting|CastToBP_GI (Game|GetGameInstance)))
    (if (Variables|/Game/Blueprints/Public/BP_GI.BP_GI_C|GetIsDebugMode _asbp_gi)
      (CallFunction|RestartGame))))

(event Input|KeyboardEvents|End
  (params (Key :type Key%20Structure))
  ;[1 0.8557 0] for debug
  (:Pressed
    (bind _asbp_gi (Utilities|Casting|CastToBP_GI (Game|GetGameInstance)))
    (if (Variables|/Game/Blueprints/Public/BP_GI.BP_GI_C|GetIsDebugMode _asbp_gi)
      (Game|OpenLevel(byName) "Entry"))))

(event Input|KeyboardEvents|M
  (params (Key :type Key%20Structure))
  ;[1 0.8557 0] for debug
  (:Pressed
    (bind _asbp_gi (Utilities|Casting|CastToBP_GI (Game|GetGameInstance)))
    (if (Variables|/Game/Blueprints/Public/BP_GI.BP_GI_C|GetIsDebugMode _asbp_gi)
      (bind _outactors (Actor|GetAllActorsOfClass "/Game/Blueprints/System/Main/BP_MainPS.BP_MainPS_C"))
      (Development|PrintString (Utilities|String|Append "Main PS Count : " (Utilities|String|ToString(Integer) (Utilities|Array|Length _outactors))) true true "(R=1.000000,G=0.414395,B=0.000000,A=1.000000)" 2e+01))))

(event Input|KeyboardEvents|G
  (params (Key :type Key%20Structure))
  ;[1 0.8557 0] for debug
  ;;[1 1 1] 모든 플레이어에게 대미지
  (:Pressed
    (bind _asbp_gi (Utilities|Casting|CastToBP_GI (Game|GetGameInstance)))
    (if (Variables|/Game/Blueprints/Public/BP_GI.BP_GI_C|GetIsDebugMode _asbp_gi)
      (Utilities|IsValid (Game|GetGameMode)
        (:Is%20Valid
          (bind _outactors (Actor|GetAllActorsOfClass "BP_MainPC_C"))
          (for _array_element _outactors
            (bind _asbp_main_ps (Utilities|Casting|CastToBP_MainPS (Variables|/Script/Engine.Controller|GetPlayerState _array_element)))
            (Game|Damage|ApplyDamage (Variables|/Script/Engine.PlayerState|GetPawnPrivate _asbp_main_ps) 3e+01 0 0)))))))

(event Input|KeyboardEvents|MotionControllerRightThumbstickLeft
  (params (Key :type Key%20Structure))
  ;[1 0.8557 0] for debug
  (:Pressed
    (bind _asbp_gi (Utilities|Casting|CastToBP_GI (Game|GetGameInstance)))
    (if (Variables|/Game/Blueprints/Public/BP_GI.BP_GI_C|GetIsDebugMode _asbp_gi)
      (CallFunction|ShowResult false))))

(event Input|KeyboardEvents|PageUp
  (params (Key :type Key%20Structure))
  ;[1 0.8557 0] for debug
  (:Pressed
    (bind _asbp_gi (Utilities|Casting|CastToBP_GI (Game|GetGameInstance)))
    (if (Variables|/Game/Blueprints/Public/BP_GI.BP_GI_C|GetIsDebugMode _asbp_gi)
      (CallFunction|GotoLobby))))

(event Input|KeyboardEvents|PageDown
  (params (Key :type Key%20Structure))
  ;[1 0.8557 0] for debug
  (:Pressed
    (bind _asbp_gi (Utilities|Casting|CastToBP_GI (Game|GetGameInstance)))
    (if (Variables|/Game/Blueprints/Public/BP_GI.BP_GI_C|GetIsDebugMode _asbp_gi)
      (CallFunction|RestartGame))))

(event Input|KeyboardEvents|Insert
  (params (Key :type Key%20Structure))
  ;[1 0.8557 0] for debug
  (:Pressed
    (bind _asbp_gi (Utilities|Casting|CastToBP_GI (Game|GetGameInstance)))
    (if (Variables|/Game/Blueprints/Public/BP_GI.BP_GI_C|GetIsDebugMode _asbp_gi)
      (bind _asbp_main_gs (Utilities|Casting|CastToBP_MainGS (Game|GetGameState)))
      (Default|DecreaseRespawnCount _asbp_main_gs))))

(event Input|KeyboardEvents|P
  (params (Key :type Key%20Structure))
  ;[1 0.8557 0] for debug
  (:Pressed
    (bind _asbp_gi (Utilities|Casting|CastToBP_GI (Game|GetGameInstance)))
    (if (Variables|/Game/Blueprints/Public/BP_GI.BP_GI_C|GetIsDebugMode _asbp_gi)
      (Development|PrintString (Utilities|String|Append "UID : " (Utilities|String|ToString(Integer) (Variables|/Game/Blueprints/Public/BP_GI.BP_GI_C|GetLocalUID _asbp_gi)) " SKin : " (Utilities|String|EnumtoString (Variables|/Game/Blueprints/Public/BP_GI.BP_GI_C|GetLocalSkinState _asbp_gi))) true true "(R=1.000000,G=0.124706,B=0.000000,A=1.000000)" 12.0))))

(event Input|KeyboardEvents|I
  (params (Key :type Key%20Structure))
  ;[1 0.8557 0] for debug
  (:Pressed
    (bind _asbp_gi (Utilities|Casting|CastToBP_GI (Game|GetGameInstance)))
    (if (Variables|/Game/Blueprints/Public/BP_GI.BP_GI_C|GetIsDebugMode _asbp_gi)
      (bind _asbp_main_ps (Utilities|Casting|CastToBP_MainPS (Variables|GetPlayerState)))
      (Development|PrintString (Utilities|String|Append "UID : " (Utilities|String|ToString(Integer) (Variables|/Game/Blueprints/System/Main/BP_MainPS.BP_MainPS_C|GetUID _asbp_main_ps)) " SKin : " (Utilities|String|EnumtoString (Variables|/Game/Blueprints/System/Main/BP_MainPS.BP_MainPS_C|GetSkinState _asbp_main_ps))) true true "(R=0.000000,G=1.000000,B=0.052316,A=1.000000)" 12.0))))

(event Input|KeyboardEvents|Q
  (params (Key :type Key%20Structure))
  ;[1 0.8557 0] for debug
  (:Pressed
    (bind _asbp_gi (Utilities|Casting|CastToBP_GI (Game|GetGameInstance)))
    (if (Variables|/Game/Blueprints/Public/BP_GI.BP_GI_C|GetIsDebugMode _asbp_gi)
      (CallFunction|SetMeshandMaterialAllPlayersServer))))

(event Input|KeyboardEvents|Backspace
  (params (Key :type Key%20Structure))
  ;[1 0.8557 0] for debug
  (:Pressed
    (bind _asbp_gi (Utilities|Casting|CastToBP_GI (Game|GetGameInstance)))
    (if (Variables|/Game/Blueprints/Public/BP_GI.BP_GI_C|GetIsDebugMode _asbp_gi)
      (Default|BacktoLobby _asbp_gi))))

(fn ConstructionScript
  (if (and (Pawn|IsLocalController) (Class|HeadMountedDisplayFunctionLibrary|IsHeadMountedDisplayConnected))
    (Variables|Default|SetRoleState "NewEnumerator0")
    (else
      (Variables|Default|SetRoleState "NewEnumerator1"))))

(fn SyncPlayerCurrentHPServer
  (Utilities|Array|Clear (Variables|Default|GetPlayerCurrentHP))
  (for _array_element (Variables|/Script/Engine.GameStateBase|GetPlayerArray (Game|GetGameState))
    (bind _asbp_main_ps (Utilities|Casting|CastToBP_MainPS _array_element))
    (Utilities|IsValid _asbp_main_ps
      (:Is%20Valid
        (bind _maxhp (Default|GetMaxHP _asbp_main_ps))
        (Utilities|Array|Add (Variables|Default|GetPlayerCurrentHP) (Utilities|Struct|MakePlayerHPData (Variables|/Game/Blueprints/System/Main/BP_MainPS.BP_MainPS_C|GetUID _asbp_main_ps) (Variables|/Game/Blueprints/System/Main/BP_MainPS.BP_MainPS_C|GetCurrentHP _asbp_main_ps) (Variables|/Game/Blueprints/System/Main/BP_MainPS.BP_MainPS_C|GetSkinState _asbp_main_ps) _maxhp (Variables|/Game/Blueprints/System/Main/BP_MainPS.BP_MainPS_C|GetRoleState _asbp_main_ps)))))))

(fn UpdateHunterWidgettoClient
  (params (LogOutUIDs :type Array%20of%20Integers))
  (Utilities|IsValid (Game|GetGameMode)
    (:Is%20Valid
      (bind _outactors (Actor|GetAllActorsOfClass "BP_MainPC_C"))
      (for _array_element _outactors
        (CallFunction|UpdateHunterMainWidgetClient _array_element (Variables|Default|GetPlayerCurrentHP) LogOutUIDs)))))

(fn EndLoading
  (if (Pawn|IsLocalController)
    (if (not (Variables|Default|GetEndLoadingSet))
      (if (Utilities|IsLocalHunter?)
        (CallFunction|PawnSpawn (Game|Player|GetPlayerPawn 0))
        (Utilities|IsValid (Variables|Default|GetHunterMainWidget)
          (:Is%20Not%20Valid
            (bind _returnvalue (UserInterface|CreateWidget "/Game/Blueprints/System/Main/MainWidget.MainWidget_C"))
            (UserInterface|Viewport|AddtoViewport _returnvalue 0)
            (Variables|Default|SetHunterMainWidget _returnvalue)
            (bind _returnvalue_2 (UserInterface|CreateWidget "/Game/Blueprints/HunterUI/HunterControlWidget.HunterControlWidget_C"))
            (UserInterface|Viewport|AddtoViewport _returnvalue_2 0)
            (Variables|Default|SetHunterControlWidget _returnvalue_2)
            (Variables|Default|SetEndLoadingSet true)))
        (else
          (bind _asbp_vrpawn_main (Utilities|Casting|CastToBP_VRPawnMain (Game|Player|GetPlayerPawn 0)))
          (Default|SetGameMode _asbp_vrpawn_main)
          (CallFunction|AddOctoMainWidget))))))

(fn UpdateWidget
  (params (Array :type Array%20of%20Player%20HP%20Data%20Structures) (LogOutUIDs :type Array%20of%20Integers))
  (bind _huntermainwidget (Variables|Default|GetHunterMainWidget))
  (bind _huntermainwidget_2 (Variables|Default|GetHunterMainWidget))
  (bind _huntermainwidget_3 (Variables|Default|GetHunterMainWidget))
  (bind _huntermainwidget_4 (Variables|Default|GetHunterMainWidget))
  (bind _huntermainwidget_5 (Variables|Default|GetHunterMainWidget))
  (for _array_element Array
    (LocalVariables|SetHP (/ (.CurrentHP (Utilities|Struct|BreakPlayerHPData _array_element)) (.MaxHP (Utilities|Struct|BreakPlayerHPData _array_element))))
    (LocalVariables|SetUID (.UID (Utilities|Struct|BreakPlayerHPData _array_element)))
    (LocalVariables|SetSkinState (.SkinState (Utilities|Struct|BreakPlayerHPData _array_element)))
    (if (not (== (LocalVariables|GetUID) -1))
      ;[1 1 1] Octo HP 동기화
      (if (and (== (LocalVariables|GetUID) 0) (Utilities|Enum|Equal(Enum) (.RoleState (Utilities|Struct|BreakPlayerHPData _array_element)) "NewEnumerator0"))
        (Utilities|IsValid _huntermainwidget
          (:Is%20Valid
            (Default|SetOctoHPBarPercent _huntermainwidget (LocalVariables|GetHP))))
        (else
          ;[1 1 1] 헌터 로컬 플레이어 HP 동기화
          (bind _asbp_main_ps (Utilities|Casting|CastToBP_MainPS (Variables|GetPlayerState)))
          (Utilities|IsValid _asbp_main_ps
            (:Is%20Valid
              (if (== (LocalVariables|GetUID) (Variables|/Game/Blueprints/System/Main/BP_MainPS.BP_MainPS_C|GetUID _asbp_main_ps))
                (Utilities|IsValid _huntermainwidget_2
                  (:Is%20Valid
                    (Default|SetHunterHPBarPercent _huntermainwidget_2 (LocalVariables|GetHP))
                    (bind (_isunderwater _isunderdeadwater) (Default|IsUnderWater _asbp_main_ps))
                    (Default|SetWaterState _huntermainwidget_2 _isunderdeadwater)
                    (Default|ToggleUnderWater _huntermainwidget_2 (or _isunderwater _isunderdeadwater))
                    (if (<= (LocalVariables|GetHP) 0.0)
                      (Default|SetTriggerOff (Variables|Default|GetHunterControlWidget)))))
                (else
                  ;[1 1 1] 서브위젯1
                  (Utilities|IsValid _huntermainwidget_4
                    (:Is%20Valid
                      (bind _isthissubwidget_suid (CallFunction|UpdateSubWidget (Variables|/Game/Blueprints/System/Main/MainWidget.MainWidget_C|GetSubHPWidget1 _huntermainwidget_4) (LocalVariables|GetUID) (LocalVariables|GetSkinState) (LocalVariables|GetHP) LogOutUIDs))
                      (if (not _isthissubwidget_suid)
                        ;[1 1 1] 서브위젯2
                        (Utilities|IsValid _huntermainwidget_5
                          (:Is%20Valid
                            (bind _isthissubwidget_suid_2 (CallFunction|UpdateSubWidget (Variables|/Game/Blueprints/System/Main/MainWidget.MainWidget_C|GetSubHPWidget2 _huntermainwidget_5) (LocalVariables|GetUID) (LocalVariables|GetSkinState) (LocalVariables|GetHP) LogOutUIDs))
                            (if (not _isthissubwidget_suid_2)
                              ;[1 1 1] 서브위젯3
                              (Utilities|IsValid _huntermainwidget_3
                                (:Is%20Valid
                                  (CallFunction|UpdateSubWidget (Variables|/Game/Blueprints/System/Main/MainWidget.MainWidget_C|GetSubHPWidget3 _huntermainwidget_3) (LocalVariables|GetUID) (LocalVariables|GetSkinState) (LocalVariables|GetHP) LogOutUIDs))))))))))))))))))

(fn UpdateSubWidget
  (params (SubHPWidget :type Sub%20HP%20Widget%20Object%20Reference) (UID :type Integer) (SkinState :type ESkinState%20Enum :default "NewEnumerator0") (HP :type Float%20%28single-precision%29) (LogOutUIDs :type Array%20of%20Integers))
  (bind _returnvalue (== (Variables|/Game/Blueprints/System/Main/SubHPWidget.SubHPWidget_C|GetUID SubHPWidget) UID))
  (Utilities|IsValid SubHPWidget
    (:Is%20Valid
      (if (Variables|/Game/Blueprints/System/Main/SubHPWidget.SubHPWidget_C|GetIsSet SubHPWidget)
        (if _returnvalue
          (if (Variables|/Game/Blueprints/System/Main/SubHPWidget.SubHPWidget_C|GetIsLogout SubHPWidget)
            _
            (elif (Utilities|Array|ContainsItem LogOutUIDs (Variables|/Game/Blueprints/System/Main/SubHPWidget.SubHPWidget_C|GetUID SubHPWidget))
              (Default|LogOut SubHPWidget)
              (else
                (Default|SetSubHPBarPercent SubHPWidget HP :!label _label)))))
        (else
          (Default|SetUID SubHPWidget UID)
          (bind _result (Default|GetSkinStruct (Variables|Default|GetBP_SkinData) SkinState))
          (Default|SetPortrait SubHPWidget (.Portrait (Utilities|Struct|BreakSkinStruct _result)))
          (goto _label)))
      (return _returnvalue))))

(fn SpawnHunter
  (bind _playerstate (Variables|GetPlayerState))
  (bind _pawnprivate (Variables|/Script/Engine.PlayerState|GetPawnPrivate _playerstate))
  (Utilities|IsValid _playerstate
    (:Is%20Valid
      ;[1 1 1] 실패했을 때만
      (Utilities|IsValid _pawnprivate
        (:Is%20Valid
          (bind _asbp_player_character_sn (Utilities|Casting|CastToBP_PlayerCharacter_SN _pawnprivate)
            (:then
              (Utilities|IsValid _asbp_player_character_sn
                (:Is%20Not%20Valid
                  _)))
            (:CastFailed
              _)))
        (:Is%20Not%20Valid
          _))
      (bind _asbp_main_ps (Utilities|Casting|CastToBP_MainPS (Variables|GetPlayerState)))
      (Utilities|IsValid _asbp_main_ps
        (:Is%20Valid
          (Default|SpawnHunter _asbp_main_ps)
          (return))))))